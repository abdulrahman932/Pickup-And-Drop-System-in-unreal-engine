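; Hand inventory component for BP_ThirdPersonCharacter that lets it hold, drop and place one item per hand.
; Pickup fills the right hand by default, or the left when Ctrl is set or the right is full, attaching the item to that mesh grip socket.
; DropItem detaches the chosen hand's item, with OnGround toggled on pickup and drop.
; PlaceItem passes the item to a target actor through a PlaceObject message and clears that hand.
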(event EventBeginPlay)

(event EventTick
  (params (DeltaSeconds :type Float%20%28single-precision%29)))

(fn Pickup
  (params (Item :type Actor%20Object%20Reference) (ctrl :type Boolean))
  (bind _output_get (Variables|Default|SetCurrenItem Item))
  (Utilities|IsValid _output_get
    (:Is%20Valid
      (switch Utilities|FlowControl|Switch|SwitchonE_Hand "NewEnumerator0"
        (:NewEnumerator0
          (if ctrl
            (switch Utilities|FlowControl|Switch|SwitchonE_Hand "NewEnumerator1" :!label _label
              (:NewEnumerator1
                (Utilities|IsValid (Variables|Default|GetLeftHandItem)
                  (:Is%20Valid
                    (Development|PrintString "left hand is occupied")
                    (return))
                  (:Is%20Not%20Valid
                    (bind _asbp_pickup_item (Utilities|Casting|CastToBP_PickupItem (Variables|Default|GetCurrenItem)))
                    (Variables|/Game/Pickup/BP_PickupItem.BP_PickupItem_C|SetOnGround _asbp_pickup_item false)
                    (bind _asbp_third_person_character (Utilities|Casting|CastToBP_ThirdPersonCharacter (Components|GetOwner)))
                    (Transformation|AttachComponentToComponent (Variables|Default|GetCurrenItem) (Variables|/Script/Engine.Character|GetMesh _asbp_third_person_character) "HandGrip_L" "SnapToTarget" "SnapToTarget" "KeepWorld" true)
                    (Variables|Default|SetLeftHandItem (Variables|Default|GetCurrenItem))))))
            (else
              (Utilities|IsValid (Variables|Default|GetRightHandItem)
                (:Is%20Valid
                  (goto _label))
                (:Is%20Not%20Valid
                  (bind _asbp_pickup_item_2 (Utilities|Casting|CastToBP_PickupItem (Variables|Default|GetCurrenItem)))
                  (Variables|/Game/Pickup/BP_PickupItem.BP_PickupItem_C|SetOnGround _asbp_pickup_item_2 false)
                  (bind _asbp_third_person_character_2 (Utilities|Casting|CastToBP_ThirdPersonCharacter (Components|GetOwner)))
                  (Transformation|AttachComponentToComponent (Variables|Default|GetCurrenItem) (Variables|/Script/Engine.Character|GetMesh _asbp_third_person_character_2) "HandGrip_R" "SnapToTarget" "SnapToTarget" "KeepWorld" true)
                  (Variables|Default|SetRightHandItem (Variables|Default|GetCurrenItem)))))))))
    (:Is%20Not%20Valid
      (Development|PrintString "hand oqupide")
      (return))))

(fn DropItem
  (params (RightOrLeft :type Boolean))
  (Utilities|IsValid (select RightOrLeft (Variables|Default|GetLeftHandItem) (Variables|Default|GetRightHandItem))
    (:Is%20Valid
      (Transformation|DetachFromActor (select RightOrLeft (Variables|Default|GetLeftHandItem) (Variables|Default|GetRightHandItem)) "KeepWorld" "KeepWorld" "KeepWorld")
      (bind _asbp_pickup_item (Utilities|Casting|CastToBP_PickupItem (select RightOrLeft (Variables|Default|GetLeftHandItem) (Variables|Default|GetRightHandItem))))
      (Variables|/Game/Pickup/BP_PickupItem.BP_PickupItem_C|SetOnGround _asbp_pickup_item true)
      (if RightOrLeft
        (Variables|Default|SetLeftHandItem 0)
        (else
          (Variables|Default|SetRightHandItem 0))))))

(fn PlaceItem
  (params (actor :type Actor%20Object%20Reference) (rightOrLeft :type Boolean))
  (Utilities|IsValid (select rightOrLeft (Variables|Default|GetLeftHandItem) (Variables|Default|GetRightHandItem))
    (:Is%20Valid
      (Class|BPIIntract|PlaceObject(Message) actor (select rightOrLeft (Variables|Default|GetLeftHandItem) (Variables|Default|GetRightHandItem)))
      (if rightOrLeft
        (Variables|Default|SetLeftHandItem 0)
        (else
          (Variables|Default|SetRightHandItem 0))))))